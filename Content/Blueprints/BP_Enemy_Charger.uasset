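; BP_Enemy_Charger is an ant enemy that roams at random and charges the player on sight.
; Tick with a random Delay drives roaming unless IsChasing, which this graph never sets.
; PawnSensing starts a move to the player, chirping on first sighting and dealing damage on arrival.
; Hits flash a damaged material, death spawns gore, effects and sound, and destruction calls a mob-count dispatcher.
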(event OnSeePawn(PawnSensing)
  (params (Pawn :type Pawn%20Object%20Reference))
  ;[1 1 1] If sees player try to move and attack
  (bind _asfirst_person_character (Utilities|Casting|CastToFirstPersonCharacter Pawn))
  (AI|AIMoveTo self "0, 0, 0" _asfirst_person_character 5.0 false
    (:then
      (if (not (Variables|Default|GetsoundTriggered))
        (Audio|PlaySoundatLocation "/Game/Music/chirp1_Cue.chirp1_Cue" (Transformation|GetWorldLocation (Variables|Collision|GetCapsuleComponent)) "0, 0, 0" 1.0 1.0 0.0 0 0 0)
        (Variables|Default|SetsoundTriggered true)))
    (:OnSuccess
      (Game|Damage|ApplyDamage (Game|GetPlayerCharacter 0) 2.0 0 0)
      (Audio|PlaySoundatLocation "/Game/Music/chirp2_Cue.chirp2_Cue" (Transformation|GetWorldLocation (Variables|Collision|GetCapsuleComponent)) "0, 0, 0" 1.0 1.0 0.0 0 0 0)
      (Utilities|FlowControl|Delay 0.1))))

(event EventTick
  (params (DeltaSeconds :type Float%20%28single-precision%29))
  ;[1 1 1] Ai random roam when not chasing player
  (Utilities|FlowControl|Delay (Math|Random|RandomFloatinRange 2.0 5.0))
  (Variables|Default|SetisMoving true)
  (if (Variables|Default|GetisChasing)
    (Variables|Default|SetisMoving false)
    (else
      (AI|AIMoveTo self (.RandomLocation (AI|Navigation|GetRandomReachablePointinRadius (Transformation|GetActorLocation) 1.5e+03 0 0)) 0 5.0 false
        (:OnSuccess
          _)
        (:OnFail
          _))
      (Variables|Default|SetisMoving false))))

(event EventBeginPlay
  ;[1 1 1] Init vars
  (Variables|Default|SetCurrentHP (Variables|Default|GetMaxHP)))

(event Game|Damage|EventAnyDamage
  (params (Damage :type Float%20%28single-precision%29) (DamageType :type Damage%20Type%20Object%20Reference) (InstigatedBy :type Controller%20Object%20Reference) (DamageCauser :type Actor%20Object%20Reference))
  ;[1 1 1] Take damage and death check
  (bind _output_get (Variables|Default|SetCurrentHP (- (Variables|Default|GetCurrentHP) Damage)))
  (if (<= _output_get 0.0)
    (Game|SpawnActorfromClass "/Game/Blueprints/BP_Enemy_Charger_Gore.BP_Enemy_Charger_Gore_C" (Transformation|GetActorTransform self) "AlwaysSpawn" 0 0)
    (Niagara|SpawnSystematLocation "/Game/Effects/DeathSystem.DeathSystem" (Transformation|GetActorLocation))
    (Audio|PlaySoundatLocation "/Game/Music/chirp3_Cue.chirp3_Cue" (Transformation|GetWorldLocation (Variables|Collision|GetCapsuleComponent)) "0, 0, 0" 1.0 1.0 0.0 0 0 0)
    (Actor|DestroyActor)
    (else
      (Audio|PlaySoundatLocation "/Game/Music/chirp_Damaged.chirp_Damaged" (Transformation|GetWorldLocation (Variables|Collision|GetCapsuleComponent)) "0, 0, 0" 1.0 1.0 0.0 0 0 0)
      (Rendering|Material|SetMaterial (Variables|Default|GetStaticMesh) 0 "/Game/AntDamaged1.AntDamaged1")
      (Utilities|FlowControl|Delay 0.2)
      (Rendering|Material|SetMaterial (Variables|Default|GetStaticMesh) 0 "/Game/Objects/Textures/Ant.Ant"))))

(event EventDestroyed
  ;[1 1 1] Updates level blueprint mob counter
  (Default|CallMobCountDispatcher))

(fn ConstructionScript)