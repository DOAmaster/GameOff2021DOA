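; Charger enemy (Gore variant) Blueprint whose event graph is inert: every event is empty and all logic is disconnected.
; The unwired nodes sketch random roaming, chasing a seen player with chirp and melee damage, and HP-based death with effects.
; They also hold a damage material flash and a mob-count dispatcher call.
; As written, this graph runs none of that behavior.
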(event OnSeePawn(PawnSensing)
  (params (Pawn :type Pawn%20Object%20Reference))
  ;[1 1 1] If sees player try to move and attack
)

(event EventTick
  (params (DeltaSeconds :type Float%20%28single-precision%29))
  ;[1 1 1] Ai random roam when not chasing player
)

(event EventBeginPlay
  ;[1 1 1] Init vars
)

(event Game|Damage|EventAnyDamage
  (params (Damage :type Float%20%28single-precision%29) (DamageType :type Damage%20Type%20Object%20Reference) (InstigatedBy :type Controller%20Object%20Reference) (DamageCauser :type Actor%20Object%20Reference))
  ;[1 1 1] Take damage and death check
)

(event EventDestroyed
  ;[1 1 1] Updates level blueprint mob counter
)

(fn ConstructionScript)