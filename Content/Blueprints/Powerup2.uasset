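; Movement speed pickup that permanently raises the first-person character's walk speed in ranked tiers.
; On box overlap it switches on the character's MoveSpeedRank, setting a higher MaxWalkSpeed, incrementing the rank and updating PowerUpString2 with a label or added "+".
; Upgrades set AlertText on player 0's character and destroy the pickup; at max rank it only prints a message and destroys itself.
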(event OnComponentBeginOverlap(Box)
  (params (OverlappedComponent :type Primitive%20Component%20Object%20Reference) (OtherActor :type Actor%20Object%20Reference) (OtherComp :type Primitive%20Component%20Object%20Reference) (OtherBodyIndex :type Integer) (bFromSweep :type Boolean) (SweepResult :type Hit%20Result%20Structure%20%28by%20ref%29))
  (bind _asfirst_person_character (Utilities|Casting|CastToFirstPersonCharacter OtherActor))
  ;[1 1 1] Walk Speed Ranks
  (Development|PrintString "Attackspeed up")
  (switch int (Variables|/Game/FirstPersonBP/Blueprints/FirstPersonCharacter.FirstPersonCharacter_C|GetMoveSpeedRank _asfirst_person_character)
    (:0
      (Variables|/Game/FirstPersonBP/Blueprints/FirstPersonCharacter.FirstPersonCharacter_C|SetPowerUpString2 _asfirst_person_character "Crawl Speed")
      (Variables|/Script/Engine.CharacterMovementComponent|SetMaxWalkSpeed (Variables|/Script/Engine.Character|GetCharacterMovement _asfirst_person_character) 8e+02)
      (Math|Integer|IncrementInt (Variables|/Game/FirstPersonBP/Blueprints/FirstPersonCharacter.FirstPersonCharacter_C|GetMoveSpeedRank _asfirst_person_character)
        (:%20%20
          (bind _asfirst_person_character_2 (Utilities|Casting|CastToFirstPersonCharacter (Game|Player|GetPlayerPawn 0) :!label _label))
          (Variables|/Game/FirstPersonBP/Blueprints/FirstPersonCharacter.FirstPersonCharacter_C|SetAlertText _asfirst_person_character_2 "Speed Increased")
          (Actor|DestroyActor))))
    (:1
      (Variables|/Game/FirstPersonBP/Blueprints/FirstPersonCharacter.FirstPersonCharacter_C|SetPowerUpString2 _asfirst_person_character (Utilities|String|Append (Variables|/Game/FirstPersonBP/Blueprints/FirstPersonCharacter.FirstPersonCharacter_C|GetPowerUpString2 _asfirst_person_character) "+"))
      (Variables|/Script/Engine.CharacterMovementComponent|SetMaxWalkSpeed (Variables|/Script/Engine.Character|GetCharacterMovement _asfirst_person_character) 9e+02)
      (Math|Integer|IncrementInt (Variables|/Game/FirstPersonBP/Blueprints/FirstPersonCharacter.FirstPersonCharacter_C|GetMoveSpeedRank _asfirst_person_character)
        (:%20%20
          (goto _label))))
    (:2
      (Variables|/Game/FirstPersonBP/Blueprints/FirstPersonCharacter.FirstPersonCharacter_C|SetPowerUpString2 _asfirst_person_character (Utilities|String|Append (Variables|/Game/FirstPersonBP/Blueprints/FirstPersonCharacter.FirstPersonCharacter_C|GetPowerUpString2 _asfirst_person_character) "+"))
      (Variables|/Script/Engine.CharacterMovementComponent|SetMaxWalkSpeed (Variables|/Script/Engine.Character|GetCharacterMovement _asfirst_person_character) 1e+03)
      (Math|Integer|IncrementInt (Variables|/Game/FirstPersonBP/Blueprints/FirstPersonCharacter.FirstPersonCharacter_C|GetMoveSpeedRank _asfirst_person_character)
        (:%20%20
          (goto _label))))
    (:3
      (Variables|/Game/FirstPersonBP/Blueprints/FirstPersonCharacter.FirstPersonCharacter_C|SetPowerUpString2 _asfirst_person_character (Utilities|String|Append (Variables|/Game/FirstPersonBP/Blueprints/FirstPersonCharacter.FirstPersonCharacter_C|GetPowerUpString2 _asfirst_person_character) "+"))
      (Variables|/Script/Engine.CharacterMovementComponent|SetMaxWalkSpeed (Variables|/Script/Engine.Character|GetCharacterMovement _asfirst_person_character) 1.1e+03)
      (Math|Integer|IncrementInt (Variables|/Game/FirstPersonBP/Blueprints/FirstPersonCharacter.FirstPersonCharacter_C|GetMoveSpeedRank _asfirst_person_character)
        (:%20%20
          (goto _label))))
    (:4
      (Development|PrintString "Move Speed maxed")
      (Actor|DestroyActor))))

(event EventBeginPlay)

(event Collision|EventActorBeginOverlap
  (params (OtherActor :type Actor%20Object%20Reference)))

(event EventTick
  (params (DeltaSeconds :type Float%20%28single-precision%29)))

(fn ConstructionScript)