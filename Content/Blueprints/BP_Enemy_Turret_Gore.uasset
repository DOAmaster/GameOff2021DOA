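; BP_Enemy_Turret_Gore is an enemy turret gore actor with no active graph logic, apparently duplicated from a turret enemy.
; BeginPlay, AnyDamage and the construction script are empty.
; Disconnected leftovers hold turret behavior: health setup, facing the player, timed projectile firing with an impulse, and damage handling.
; The unused death branch spawns this gore class, calls a mob count dispatcher and destroys the actor.
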(event EventBeginPlay
  ;[1 1 1] INIT vars
)

(event Game|Damage|EventAnyDamage
  (params (Damage :type Float%20%28single-precision%29) (DamageType :type Damage%20Type%20Object%20Reference) (InstigatedBy :type Controller%20Object%20Reference) (DamageCauser :type Actor%20Object%20Reference))
  ;[1 1 1] Take Damage
)

(fn ConstructionScript)