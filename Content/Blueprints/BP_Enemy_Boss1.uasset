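; Boss enemy actor that faces and shoots at the player it sees, and dies after enough hits.
; Pawn sensing turns it toward the first-person character and spawns an enemy projectile, gated by a two-second cooldown flag.
; Each damage event removes one HP, then either turns it toward the player controller's location after a short delay or, at zero, calls the mob count dispatcher and destroys it.
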(event OnSeePawn(PawnSensing)
  (params (Pawn :type Pawn%20Object%20Reference))
  (bind _asfirst_person_character (Utilities|Casting|CastToFirstPersonCharacter Pawn))
  (Utilities|FlowControl|Sequence
    (:then_0
      ;[1 1 1] Face Player
      (Transformation|SetActorRotation (Math|Rotator|FindLookatRotation (Transformation|GetActorLocation) (Transformation|GetActorLocation _asfirst_person_character))))
    (:then_1
      ;[1 1 1] Shoot at player
      (if (Variables|Default|GetSpawnProjectile)
        (bind _returnvalue (Game|SpawnActorfromClass "/Game/Blueprints/EnemyProjectile.EnemyProjectile_C" (Transformation|GetWorldTransform (Variables|Default|GetSpawnProjectileLocation)) "Undefined" 0 0))
        (Variables|Default|SetSpawnProjectile false)
        (Utilities|FlowControl|Delay 2.0)
        (Variables|Default|SetSpawnProjectile true)))))

(event EventBeginPlay
  (Variables|Default|SetCurrentHP (Variables|Default|GetMaxHP)))

(event Game|Damage|EventAnyDamage
  (params (Damage :type Float%20%28single-precision%29) (DamageType :type Damage%20Type%20Object%20Reference) (InstigatedBy :type Controller%20Object%20Reference) (DamageCauser :type Actor%20Object%20Reference))
  (Development|PrintString "Boss Hit")
  (bind _output_get (Variables|Default|SetCurrentHP (- (Variables|Default|GetCurrentHP) 1.0)))
  (if (<= _output_get 0.0)
    (Default|CallMobCountDispatcher)
    (Actor|DestroyActor)
    (else
      (Utilities|FlowControl|Delay 0.4)
      (Transformation|SetActorRotation (Math|Rotator|FindLookatRotation (Transformation|GetActorLocation) (Transformation|GetActorLocation (Game|GetPlayerController 0)))))))

(fn ConstructionScript)