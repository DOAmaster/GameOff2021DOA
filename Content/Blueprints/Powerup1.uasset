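; Attack speed pickup that upgrades the FirstPersonCharacter that overlaps its Box, then destroys itself.
; A switch on the character's AttackSpeedRank shortens FireDelay, updates PowerUpString and increments the rank, across four tiers.
; Each upgrade also sets AlertText on player pawn 0.
; At max rank the pickup only prints a maxed message and is still consumed.
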(event OnComponentBeginOverlap(Box)
  (params (OverlappedComponent :type Primitive%20Component%20Object%20Reference) (OtherActor :type Actor%20Object%20Reference) (OtherComp :type Primitive%20Component%20Object%20Reference) (OtherBodyIndex :type Integer) (bFromSweep :type Boolean) (SweepResult :type Hit%20Result%20Structure%20%28by%20ref%29))
  (bind _asfirst_person_character (Utilities|Casting|CastToFirstPersonCharacter OtherActor))
  ;[1 1 1] Attack Speed Ranks
  (Development|PrintString "Attackspeed up")
  (switch int (Variables|/Game/FirstPersonBP/Blueprints/FirstPersonCharacter.FirstPersonCharacter_C|GetAttackSpeedRank _asfirst_person_character)
    (:0
      (Variables|/Game/FirstPersonBP/Blueprints/FirstPersonCharacter.FirstPersonCharacter_C|SetPowerUpString _asfirst_person_character "AS:+")
      (Variables|/Game/FirstPersonBP/Blueprints/FirstPersonCharacter.FirstPersonCharacter_C|SetFireDelay _asfirst_person_character 0.4)
      (Math|Integer|IncrementInt (Variables|/Game/FirstPersonBP/Blueprints/FirstPersonCharacter.FirstPersonCharacter_C|GetAttackSpeedRank _asfirst_person_character)
        (:%20%20
          (bind _asfirst_person_character_2 (Utilities|Casting|CastToFirstPersonCharacter (Game|Player|GetPlayerPawn 0) :!label _label))
          (Variables|/Game/FirstPersonBP/Blueprints/FirstPersonCharacter.FirstPersonCharacter_C|SetAlertText _asfirst_person_character_2 "Attack Speed Increased")
          (Actor|DestroyActor))))
    (:1
      (Variables|/Game/FirstPersonBP/Blueprints/FirstPersonCharacter.FirstPersonCharacter_C|SetPowerUpString _asfirst_person_character "AS:++")
      (Variables|/Game/FirstPersonBP/Blueprints/FirstPersonCharacter.FirstPersonCharacter_C|SetFireDelay _asfirst_person_character 0.3)
      (Math|Integer|IncrementInt (Variables|/Game/FirstPersonBP/Blueprints/FirstPersonCharacter.FirstPersonCharacter_C|GetAttackSpeedRank _asfirst_person_character)
        (:%20%20
          (goto _label))))
    (:2
      (Variables|/Game/FirstPersonBP/Blueprints/FirstPersonCharacter.FirstPersonCharacter_C|SetPowerUpString _asfirst_person_character "AS:+++")
      (Variables|/Game/FirstPersonBP/Blueprints/FirstPersonCharacter.FirstPersonCharacter_C|SetFireDelay _asfirst_person_character 0.2)
      (Math|Integer|IncrementInt (Variables|/Game/FirstPersonBP/Blueprints/FirstPersonCharacter.FirstPersonCharacter_C|GetAttackSpeedRank _asfirst_person_character)
        (:%20%20
          (goto _label))))
    (:3
      (Variables|/Game/FirstPersonBP/Blueprints/FirstPersonCharacter.FirstPersonCharacter_C|SetPowerUpString _asfirst_person_character "AS:++++")
      (Variables|/Game/FirstPersonBP/Blueprints/FirstPersonCharacter.FirstPersonCharacter_C|SetFireDelay _asfirst_person_character 0.01)
      (Math|Integer|IncrementInt (Variables|/Game/FirstPersonBP/Blueprints/FirstPersonCharacter.FirstPersonCharacter_C|GetAttackSpeedRank _asfirst_person_character)
        (:%20%20
          (goto _label))))
    (:4
      (Development|PrintString "Attack speed Maxed")
      (Actor|DestroyActor))))

(event EventBeginPlay)

(event Collision|EventActorBeginOverlap
  (params (OtherActor :type Actor%20Object%20Reference)))

(event EventTick
  (params (DeltaSeconds :type Float%20%28single-precision%29)))

(fn ConstructionScript)