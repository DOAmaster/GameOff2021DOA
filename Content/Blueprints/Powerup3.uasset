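; Pickup actor that upgrades the first-person character's shooting damage when the player overlaps its box.
; The overlap casts to FirstPersonCharacter and switches on its ShootDamageRank to set a fixed damage value, raise the rank and build the PowerUpString3 label with a plus per extra rank.
; The pickup destroys itself on each handled rank, including the capped one, which only prints a maxed message.
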(event OnComponentBeginOverlap(Box)
  (params (OverlappedComponent :type Primitive%20Component%20Object%20Reference) (OtherActor :type Actor%20Object%20Reference) (OtherComp :type Primitive%20Component%20Object%20Reference) (OtherBodyIndex :type Integer) (bFromSweep :type Boolean) (SweepResult :type Hit%20Result%20Structure%20%28by%20ref%29))
  (bind _asfirst_person_character (Utilities|Casting|CastToFirstPersonCharacter OtherActor))
  ;[1 1 1] Attack Damage Ranks
  (Development|PrintString "Damage Up")
  (switch int (Variables|/Game/FirstPersonBP/Blueprints/FirstPersonCharacter.FirstPersonCharacter_C|GetShootDamageRank _asfirst_person_character)
    (:0
      (Variables|/Game/FirstPersonBP/Blueprints/FirstPersonCharacter.FirstPersonCharacter_C|SetPowerUpString3 _asfirst_person_character "Damage")
      (Variables|/Game/FirstPersonBP/Blueprints/FirstPersonCharacter.FirstPersonCharacter_C|SetShootDamage _asfirst_person_character 2.0)
      (Math|Integer|IncrementInt (Variables|/Game/FirstPersonBP/Blueprints/FirstPersonCharacter.FirstPersonCharacter_C|GetShootDamageRank _asfirst_person_character)
        (:%20%20
          (Actor|DestroyActor))))
    (:1
      (Variables|/Game/FirstPersonBP/Blueprints/FirstPersonCharacter.FirstPersonCharacter_C|SetPowerUpString3 _asfirst_person_character (Utilities|String|Append (Variables|/Game/FirstPersonBP/Blueprints/FirstPersonCharacter.FirstPersonCharacter_C|GetPowerUpString3 _asfirst_person_character) "+"))
      (Variables|/Game/FirstPersonBP/Blueprints/FirstPersonCharacter.FirstPersonCharacter_C|SetShootDamage _asfirst_person_character 3.0)
      (Math|Integer|IncrementInt (Variables|/Game/FirstPersonBP/Blueprints/FirstPersonCharacter.FirstPersonCharacter_C|GetShootDamageRank _asfirst_person_character)
        (:%20%20
          (Actor|DestroyActor))))
    (:2
      (Variables|/Game/FirstPersonBP/Blueprints/FirstPersonCharacter.FirstPersonCharacter_C|SetPowerUpString3 _asfirst_person_character (Utilities|String|Append (Variables|/Game/FirstPersonBP/Blueprints/FirstPersonCharacter.FirstPersonCharacter_C|GetPowerUpString3 _asfirst_person_character) "+"))
      (Variables|/Game/FirstPersonBP/Blueprints/FirstPersonCharacter.FirstPersonCharacter_C|SetShootDamage _asfirst_person_character 4.0)
      (Math|Integer|IncrementInt (Variables|/Game/FirstPersonBP/Blueprints/FirstPersonCharacter.FirstPersonCharacter_C|GetShootDamageRank _asfirst_person_character)
        (:%20%20
          (Actor|DestroyActor))))
    (:3
      (Variables|/Game/FirstPersonBP/Blueprints/FirstPersonCharacter.FirstPersonCharacter_C|SetPowerUpString3 _asfirst_person_character (Utilities|String|Append (Variables|/Game/FirstPersonBP/Blueprints/FirstPersonCharacter.FirstPersonCharacter_C|GetPowerUpString3 _asfirst_person_character) "+"))
      (Variables|/Game/FirstPersonBP/Blueprints/FirstPersonCharacter.FirstPersonCharacter_C|SetShootDamage _asfirst_person_character 5.0)
      (Math|Integer|IncrementInt (Variables|/Game/FirstPersonBP/Blueprints/FirstPersonCharacter.FirstPersonCharacter_C|GetShootDamageRank _asfirst_person_character)
        (:%20%20
          (Actor|DestroyActor))))
    (:4
      (Development|PrintString "Spit Damage Maxed")
      (Actor|DestroyActor))))

(event EventBeginPlay)

(event Collision|EventActorBeginOverlap
  (params (OtherActor :type Actor%20Object%20Reference)))

(event EventTick
  (params (DeltaSeconds :type Float%20%28single-precision%29)))

(fn ConstructionScript)