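; BP_Bomb is a timed bomb actor that blinks faster as it counts down, then explodes and destroys itself.
; On BeginPlay, a chain of shrinking delays alternates the Sphere between two glow materials.
; At the end it activates BlastBox, spawns an Explosion actor at its transform and is destroyed.
; The BlastBox overlap event is empty, as its logic for destroying BP_BreakableRock with a sound is disconnected.
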(event OnComponentBeginOverlap(BlastBox)
  (params (OverlappedComponent :type Primitive%20Component%20Object%20Reference) (OtherActor :type Actor%20Object%20Reference) (OtherComp :type Primitive%20Component%20Object%20Reference) (OtherBodyIndex :type Integer) (bFromSweep :type Boolean) (SweepResult :type Hit%20Result%20Structure%20%28by%20ref%29)))

(event EventBeginPlay
  (Utilities|FlowControl|Delay 1.0)
  (Rendering|Material|SetMaterial (Variables|Default|GetSphere) 0 "/Game/Materials/RedDarkGlow.RedDarkGlow")
  (Utilities|FlowControl|Delay 0.5)
  (Rendering|Material|SetMaterial (Variables|Default|GetSphere) 0 "/Game/Materials/GlowingMaster.GlowingMaster")
  (Utilities|FlowControl|Delay 1.0)
  (Rendering|Material|SetMaterial (Variables|Default|GetSphere) 0 "/Game/Materials/RedDarkGlow.RedDarkGlow")
  (Utilities|FlowControl|Delay 0.5)
  (Rendering|Material|SetMaterial (Variables|Default|GetSphere) 0 "/Game/Materials/GlowingMaster.GlowingMaster")
  (Utilities|FlowControl|Delay 0.5)
  (Rendering|Material|SetMaterial (Variables|Default|GetSphere) 0 "/Game/Materials/RedDarkGlow.RedDarkGlow")
  (Utilities|FlowControl|Delay 0.5)
  (Rendering|Material|SetMaterial (Variables|Default|GetSphere) 0 "/Game/Materials/GlowingMaster.GlowingMaster")
  (Utilities|FlowControl|Delay 0.5)
  (Rendering|Material|SetMaterial (Variables|Default|GetSphere) 0 "/Game/Materials/RedDarkGlow.RedDarkGlow")
  (Utilities|FlowControl|Delay 0.1)
  (Rendering|Material|SetMaterial (Variables|Default|GetSphere) 0 "/Game/Materials/GlowingMaster.GlowingMaster")
  (Utilities|FlowControl|Delay 0.1)
  (Rendering|Material|SetMaterial (Variables|Default|GetSphere) 0 "/Game/Materials/RedDarkGlow.RedDarkGlow")
  (Components|Activation|SetActive (Variables|Default|GetBlastBox) true false)
  (Game|SpawnActorfromClass "/Game/Blueprints/Explosion.Explosion_C" (Transformation|GetActorTransform self) "Undefined" 0 0)
  (Actor|DestroyActor))

(fn ConstructionScript)