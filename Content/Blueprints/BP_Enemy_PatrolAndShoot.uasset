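; Patrolling shooter enemy that turns to a seen FirstPersonCharacter and spawns EnemyProjectile on a 1.5-second cooldown.
; Damage lowers HP, then either turns it toward the player controller's location or destroys it.
; Death and a timed despawn both call the mob-count dispatcher.
; BeginPlay picks a random patrol point, but the timeline movement and projectile impulse logic are never run.
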(event OnSeePawn(PawnSensing)
  (params (Pawn :type Pawn%20Object%20Reference))
  ;[1 1 1] Look at and shoot pawn
  (bind _asfirst_person_character (Utilities|Casting|CastToFirstPersonCharacter Pawn))
  (Utilities|FlowControl|Sequence
    (:then_0
      (Transformation|SetActorRotation (Math|Rotator|FindLookatRotation (Transformation|GetActorLocation) (Transformation|GetActorLocation _asfirst_person_character))))
    (:then_1
      (if (Variables|Default|GetSpawnProjectile)
        (bind _returnvalue (Game|SpawnActorfromClass "/Game/Blueprints/EnemyProjectile.EnemyProjectile_C" (Transformation|GetWorldTransform (Variables|Default|GetSpawnProjectileLocation)) "Undefined" 0 0))
        (Variables|Default|SetSpawnProjectile false)
        (Utilities|FlowControl|Delay 1.5)
        (Variables|Default|SetSpawnProjectile true)))))

(event EventBeginPlay
  ;[1 1 1] Set Patrol Points
  (Variables|Default|SetCurrentHP (Variables|Default|GetMaxHP))
  (Variables|Default|SetControlPoints (Utilities|Array|MakeArray (Transformation|GetWorldLocation (Variables|Default|GetMovePosition1)) (Transformation|GetWorldLocation (Variables|Default|GetMovePosition2)) (Transformation|GetWorldLocation (Variables|Default|GetMovePosition3))))
  (CallFunction|GetRandomLocation)
  (Utilities|FlowControl|Delay 25.0)
  (Development|PrintString "despawning patrol")
  (Actor|DestroyActor)
  (Default|CallMobCountDispatcher))

(event Game|Damage|EventAnyDamage
  (params (Damage :type Float%20%28single-precision%29) (DamageType :type Damage%20Type%20Object%20Reference) (InstigatedBy :type Controller%20Object%20Reference) (DamageCauser :type Actor%20Object%20Reference))
  ;[1 1 1] Taken Damage death check
  (bind _output_get (Variables|Default|SetCurrentHP (- (Variables|Default|GetCurrentHP) Damage)))
  (if (<= _output_get 0.0)
    (Default|CallMobCountDispatcher)
    (Actor|DestroyActor)
    (else
      ;[1 1 1] Alive from damage wait and rotate to player
      (Utilities|FlowControl|Delay 0.4)
      (Transformation|SetActorRotation (Math|Rotator|FindLookatRotation (Transformation|GetActorLocation) (Transformation|GetActorLocation (Game|GetPlayerController 0)))))))

(fn ConstructionScript)

(fn GetRandomLocation
  (Variables|Default|SetCurrentControlPoint (Math|Random|RandomInteger (Utilities|Array|Length (Variables|Default|GetControlPoints)))))